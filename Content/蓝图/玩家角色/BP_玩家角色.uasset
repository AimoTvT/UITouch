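; Player character pawn with Enhanced Input movement and jumping, plus a local touch UI created on possession and removed on unpossession.
; A looping timer line-traces from the camera for pawns, caching the hit as a detected car and toggling the UI's enter-vehicle button.
; Look logic exists as a custom event, but the look input action is unwired.
; A selection event applies one index across graphics quality settings and saves them.
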(event Custom|OnSelect_Event
  (params (OnIndex :type Integer))
  (bind _returnvalue (Settings|GetGameUserSettings))
  (Utilities|IsValid _returnvalue
    (:Is%20Valid
      (Utilities|FlowControl|Sequence
        (:then_0
          (Class|GameUserSettings|SetViewDistanceQuality _returnvalue OnIndex))
        (:then_1
          (Class|GameUserSettings|SetVisualEffectQuality _returnvalue OnIndex))
        (:then_2
          (Class|GameUserSettings|SetReflectionQuality _returnvalue OnIndex))
        (:then_3
          (Class|GameUserSettings|SetTextureQuality _returnvalue OnIndex))
        (:then_4
          (Class|GameUserSettings|SetPostProcessingQuality _returnvalue OnIndex))
        (:then_5
          (Class|GameUserSettings|SetShadowQuality _returnvalue OnIndex))
        (:then_6
          (Class|GameUserSettings|SetAntiAliasingQuality _returnvalue OnIndex))
        (:then_7
          (Class|GameUserSettings|SetShadingQuality _returnvalue OnIndex))
        (:then_8
          (Class|GameUserSettings|SetGlobalIlluminationQuality _returnvalue OnIndex))
        (:then_9
          (Class|GameUserSettings|SetFoliageQuality _returnvalue OnIndex))
        (:then_10
          (Class|GameUserSettings|SaveSettings _returnvalue)
          (Class|GameUserSettings|ApplySettings _returnvalue true))))))

(event Custom|添加视角
  (params (X :type Float%20%28single-precision%29) (Y :type Float%20%28double-precision%29))
  (bind _视角移动倍数 (Variables|Default|Get视角移动倍数))
  ;[0.05098 0.05098 0.05098] 视角的移动输入
  ;;[0.05098 0.05098 0.05098 1 14] 左右视角移动
  (Pawn|Input|AddControllerYawInput (* X _视角移动倍数))
  ;;[0.05098 0.05098 0.05098 1 14] 上下视角移动
  (Pawn|Input|AddControllerPitchInput (* Y _视角移动倍数)))

(event Custom|添加移动
  (params (X :type Float%20%28single-precision%29) (Y :type Float%20%28double-precision%29))
  (bind _returnvalue (Pawn|GetControlRotation :!class /Script/Engine.Pawn))
  ;[0.05098 0.05098 0.05098] 人物的移动输入
  ;;[0.05098 0.05098 0.05098 1 14] 左右的人物移动
  (Pawn|Input|AddMovementInput (Math|Vector|GetRightVector (Math|Rotator|MakeRotator (.roll _returnvalue) 0.0 (.yaw _returnvalue))) X false)
  ;;[0.05098 0.05098 0.05098 1 14] 前后的人物移动
  (Pawn|Input|AddMovementInput (Math|Vector|GetForwardVector (Math|Rotator|MakeRotator 0.0 0.0 (.yaw (Pawn|GetControlRotation :!class /Script/Engine.Pawn)))) Y false))

(event Custom|射线检查
  (bind _returnvalue (Game|GetPlayerCameraManager 0))
  (bind _tasttouchui (Variables|Default|GetTastTouchUI))
  (bind _tasttouchui_2 (Variables|Default|GetTastTouchUI))
  (bind _returnvalue_2 (Transformation|GetActorLocation _returnvalue))
  ;[1 1 1] 射线检测车辆
  (bind (_outhit _returnvalue_3) (Collision|LineTraceByChannel _returnvalue_2 (+ _returnvalue_2 (* (Transformation|GetActorForwardVector _returnvalue) 1e+03)) "TraceTypeQuery1" false 0 "None"))
  (if _returnvalue_3
    (bind _aspawn (Utilities|Casting|CastToPawn (.HitActor (Collision|BreakHitResult _outhit)))
      (:then
        (if (!= _aspawn (Variables|Default|Get检测到的车))
          (Variables|Default|Set检测到的车 _aspawn)
          (Utilities|IsValid _tasttouchui_2
            (:Is%20Valid
              (Default|上车按钮 _tasttouchui_2 true)))))
      (:CastFailed
        (Variables|Default|Set检测到的车 0 :!label _label)
        (Utilities|IsValid _tasttouchui
          (:Is%20Valid
            (Default|上车按钮 _tasttouchui false)))))
    (else
      (goto _label))))

(event Custom|跳跃
  (params (跳 :type Boolean))
  ;[0.05098 0.05098 0.05098] 跳跃的触发
  (if 跳
    (Character|Jump)
    (else
      (Character|StopJumping))))

(event Input|EnhancedActionEvents|EnhancedInputActionIA_跳
  (params (ActionValue :type Boolean) (ElapsedSeconds :type Float%20%28double-precision%29) (TriggeredSeconds :type Float%20%28double-precision%29) (InputAction :type Input%20Action%20Object%20Reference :default "/Game/蓝图/玩家角色/按键输入/按键/IA_跳.IA_跳"))
  ;[0.05098 0.05098 0.05098] 跳跃的触发
  (:Started
    (CallFunction|跳跃 true))
  (:Completed
    (CallFunction|跳跃 false)))

(event Input|EnhancedActionEvents|EnhancedInputActionIA_人物移动
  (params (ActionValue :type Vector%202D%20Structure) (ElapsedSeconds :type Float%20%28double-precision%29) (TriggeredSeconds :type Float%20%28double-precision%29) (InputAction :type Input%20Action%20Object%20Reference :default "/Game/蓝图/玩家角色/按键输入/按键/IA_人物移动.IA_人物移动"))
  ;[0.05098 0.05098 0.05098] 人物的移动输入
  (CallFunction|添加移动 (.x ActionValue) (.y ActionValue)))

(event Input|EnhancedActionEvents|EnhancedInputActionIA_视角移动
  (params (ActionValue :type Vector%202D%20Structure) (ElapsedSeconds :type Float%20%28double-precision%29) (TriggeredSeconds :type Float%20%28double-precision%29) (InputAction :type Input%20Action%20Object%20Reference :default "/Game/蓝图/玩家角色/按键输入/按键/IA_视角移动.IA_视角移动"))
  ;[0.05098 0.05098 0.05098] 视角的移动输入
)

(event EventPossessed
  (params (NewController :type Controller%20Object%20Reference))
  ;[1 1 1] 控制器开始控制时显示UI
  (|CallParentFunction NewController)
  (if (Pawn|IsLocalController NewController)
    (bind _as玩家控制器 (Utilities|Casting|CastToPlayerController NewController))
    (bind _returnvalue (UserInterface|CreateWidget "/Game/蓝图/玩家角色/BP_玩家触控UI.BP_玩家触控UI_C" _as玩家控制器))
    (Variables|Default|SetTastTouchUI _returnvalue)
    (UserInterface|Viewport|AddtoViewport _returnvalue 0)
    (Variables|/Script/Engine.PlayerController|SetbShowMouseCursor _as玩家控制器 true)
    (Input|SetInputModeGameandUI _as玩家控制器 _returnvalue "DoNotLock" false false)))

(event EventUnpossessed
  (params (OldController :type Controller%20Object%20Reference))
  (bind _tasttouchui (Variables|Default|GetTastTouchUI))
  ;[1 1 1] 控制器取消控制后删除ui
  (|CallParentFunction OldController)
  (if (Pawn|IsLocalController OldController)
    (Utilities|IsValid _tasttouchui
      (:Is%20Valid
        (Widget|RemovefromParent _tasttouchui)))))

(event EventBeginPlay
  ;[0.05098 0.05098 0.05098] 添加输入设置
  (bind _as玩家控制器 (Utilities|Casting|CastToPlayerController (Pawn|GetController)))
  (Utilities|IsValid (PlayerController|LocalPlayerSubsystems|GetEnhancedInputLocalPlayerSubsystem _as玩家控制器)
    (:Is%20Valid
      (Input|AddMappingContext (PlayerController|LocalPlayerSubsystems|GetEnhancedInputLocalPlayerSubsystem _as玩家控制器) "/Game/蓝图/玩家角色/按键输入/IMC_按键组合.IMC_按键组合" 0 "(bIgnoreAllPressedKeysUntilRelease=True,bForceImmediately=False,bNotifyUserSettings=False)"))
    (:Is%20Not%20Valid
      _))
  ;[1 1 1] 射线检测车辆
  (Utilities|Time|SetTimerbyEvent (delegate Custom|射线检查) 0.5 true))

(fn ConstructionScript)